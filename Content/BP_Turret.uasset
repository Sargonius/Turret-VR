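; Twin-gun turret that fires a BP_Projectile from its left or right shoot point along that point's forward vector.
; Each shot rumbles the controller motors on the matching side and plays a timeline that drives the gun's X position and muzzle light intensity.
; ShootEvent fires both guns, but its looping timer is unconnected, so nothing in this file triggers shooting.
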(event Custom|Shoot
  (params (LeftHand :type Boolean))
  (bind _gunleft (Variables|Default|GetGunLeft))
  (bind _shootpointleft (Variables|Default|GetShootPointLeft))
  (bind _shootpointright (Variables|Default|GetShootPointRight))
  (bind _gunright (Variables|Default|GetGunRight))
  (bind _relativelocation (Variables|/Script/Engine.SceneComponent|GetRelativeLocation _gunleft))
  (bind _relativelocation_2 (Variables|/Script/Engine.SceneComponent|GetRelativeLocation _gunright))
  (if LeftHand
    ;[1 1 1] Left
    (bind _returnvalue (Game|SpawnActorfromClass "/Game/BP_Projectile.BP_Projectile_C" (Math|Transform|MakeTransform (Transformation|GetWorldLocation _shootpointleft)) "AlwaysSpawn" 0 0))
    (Default|Fire _returnvalue (Math|Vector|GetForwardVector _shootpointleft))
    (Utilities|FlowControl|Sequence
      (:then_0
        (Game|Feedback|PlayDynamicForceFeedback (Game|GetPlayerController 0) 1.0 0.2 true true false false))
      (:then_1
        (bind (_direction _x _light) (Timeline|Timeline_1 PlayFromStart)
          (:Update
            (Transformation|SetRelativeLocation _gunleft (Math|Vector|MakeVector _x (.y _relativelocation) (.z _relativelocation)) false false)
            (Rendering|Components|Light|SetIntensity (Variables|Default|GetLightLeft) _light)))))
    (else
      ;[1 1 1] Shoot Right
      (bind _returnvalue_2 (Game|SpawnActorfromClass "/Game/BP_Projectile.BP_Projectile_C" (Math|Transform|MakeTransform (Transformation|GetWorldLocation _shootpointright)) "AlwaysSpawn" 0 0))
      (Default|Fire _returnvalue_2 (Math|Vector|GetForwardVector _shootpointright))
      (Utilities|FlowControl|Sequence
        (:then_0
          (Game|Feedback|PlayDynamicForceFeedback (Game|GetPlayerController 0) 1.0 0.2 false false true true))
        (:then_1
          (bind (_direction_2 _x_2 _light_2) (Timeline|Timeline_0 PlayFromStart)
            (:Update
              (Transformation|SetRelativeLocation _gunright (Math|Vector|MakeVector _x_2 (.y _relativelocation_2) (.z _relativelocation_2)) false false)
              (Rendering|Components|Light|SetIntensity (Variables|Default|GetLightRight) _light_2))))))))

(event Custom|Shoot%20Event
  (CallFunction|Shoot false)
  (CallFunction|Shoot true))

(event EventBeginPlay)

(fn ConstructionScript)