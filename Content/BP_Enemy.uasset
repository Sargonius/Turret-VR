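; BP_Enemy is an enemy actor that pursues the player's MotionControllerPawn and takes damage when hit.
; BeginPlay caches the first such pawn as Target.
; While 1000 units or farther, Tick lerps toward it by DeltaSeconds without sweep and turns to face it; closer, it calls Shoot every tick, currently an empty stub.
; HitBox hits deal fixed damage to Health, destroying the actor when depleted.
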(event OnComponentHit(HitBox)
  (params (HitComponent :type Primitive%20Component%20Object%20Reference) (OtherActor :type Actor%20Object%20Reference) (OtherComp :type Primitive%20Component%20Object%20Reference) (NormalImpulse :type Vector :default "0, 0, 0") (Hit :type Hit%20Result%20Structure%20%28by%20ref%29))
  (CallFunction|TakeDamage 5.0))

(event Custom|Find%20Player
  (bind _outactors (Actor|GetAllActorsOfClass "/Game/VirtualRealityBP/Blueprints/MotionControllerPawn.MotionControllerPawn_C"))
  (Variables|Default|SetTarget (Utilities|Array|Get(acopy) _outactors)))

(event Custom|Shoot)

(event Custom|Take%20Damage
  (params (Damage :type Float%20%28single-precision%29))
  (if (<= (- (Variables|Default|GetHealth) Damage) 0.0)
    (Actor|DestroyActor)
    (else
      (Variables|Default|SetHealth (- (Variables|Default|GetHealth) Damage)))))

(event EventBeginPlay
  (CallFunction|FindPlayer))

(event EventTick
  (params (DeltaSeconds :type Float%20%28single-precision%29))
  (bind _returnvalue (Transformation|GetActorLocation))
  (bind _target (Variables|Default|GetTarget))
  (bind _returnvalue_2 (Transformation|GetActorLocation _target))
  (Utilities|IsValid _target
    (:Is%20Valid
      (if (>= (Transformation|GetDistanceTo _target) 1e+03)
        (Transformation|SetActorLocation (Math|Vector|Lerp(Vector) _returnvalue _returnvalue_2 DeltaSeconds) false false)
        (Transformation|SetActorRotation (Math|Rotator|FindLookatRotation _returnvalue _returnvalue_2))
        (else
          (CallFunction|Shoot))))))

(fn ConstructionScript)