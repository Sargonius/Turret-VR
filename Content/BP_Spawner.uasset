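; BP_Spawner is an actor that keeps one BP_Enemy alive at its own location.
; A random-delay timer starts on BeginPlay and calls Spawn, which rearms itself with a new random delay each time.
; Spawn creates a new enemy at the root component's transform only when the previously spawned one is no longer valid.
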(event Custom|Spawn
  (Utilities|IsValid (Variables|Default|GetSpawnedActor)
    (:Is%20Valid
      _)
    (:Is%20Not%20Valid
      (bind _returnvalue (Game|SpawnActorfromClass "/Game/BP_Enemy.BP_Enemy_C" (Transformation|GetWorldTransform (Variables|Default|GetDefaultSceneRoot)) "Undefined" 0 0))
      (Variables|Default|SetSpawnedActor _returnvalue)))
  (Utilities|Time|SetTimerbyEvent (delegate Custom|Spawn) (Math|Random|RandomFloatinRange 2.0 5.0)))

(event EventBeginPlay
  (Utilities|Time|SetTimerbyEvent (delegate Custom|Spawn) (Math|Random|RandomFloatinRange 2.0 5.0)))

(fn ConstructionScript)